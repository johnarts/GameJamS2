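; Test pickup actor that the player grabs through an Interact event.
; On interaction it disables its mesh collision, snaps itself to the player character mesh's "ws" socket and marks itself picked up.
; It then casts the game mode to FirstPersonGameModeWithInventory and sets InventorySlot to 1 if it is 0.
; An unconnected node that would clear CurrentInventory never runs.
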(event EventInteract
  (Collision|SetCollisionEnabled (Variables|Default|GetStaticMesh) "NoCollision")
  (Transformation|AttachComponentToComponent (Variables|/Script/Engine.Character|GetMesh (Game|GetPlayerCharacter 0)) "ws" "SnapToTarget" "SnapToTarget" "KeepWorld" true)
  (Variables|Default|SetisPickedUp true)
  (bind _asfirst_person_game_mode_with_inventory (Utilities|Casting|CastToFirstPersonGameModeWithInventory (Game|GetGameMode)))
  (if (== (Variables|/Game/FirstPersonBP/Blueprints/FirstPersonGameModeWithInventory.FirstPersonGameModeWithInventory_C|GetInventory%20Slot _asfirst_person_game_mode_with_inventory) 0)
    (Variables|/Game/FirstPersonBP/Blueprints/FirstPersonGameModeWithInventory.FirstPersonGameModeWithInventory_C|SetInventory%20Slot _asfirst_person_game_mode_with_inventory 1)))

(fn ConstructionScript)