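; Interactable door actor that swings open away from or toward a chosen side and closes again on Interact.
; Opening compares the door mesh's relative Y with player 0's world Y to choose one of two opposite quarter-turn targets.
; A timeline plays forward to open and reverses to close, lerping DoorRecentered's world rotation and toggling IsOpen when finished.
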(event EventBeginPlay)

(event Collision|EventActorBeginOverlap
  (params (OtherActor :type Actor%20Object%20Reference)))

(event EventTick
  (params (DeltaSeconds :type Float%20%28single-precision%29)))

(event EventInteract
  (if (Variables|Default|Getis%20open)
    (bind _driver (Timeline|Timeline%20-%20Door%20Driven Reverse)
      (:Update
        (Transformation|SetWorldRotation (Variables|Default|GetdoorRecentered) (Math|Rotator|Lerp(Rotator) (Variables|DoorSetup|GetDoor%20Start) (Variables|DoorSetup|GetDoor%20Stop) _driver) false false))
      (:Finished
        (Variables|Default|Setis%20open (not (Variables|Default|Getis%20open)))))
    (elif (>= (.y (Variables|/Script/Engine.SceneComponent|GetRelativeLocation (Variables|Default|GetdoorRecentered))) (.y (Transformation|GetActorLocation (Game|GetPlayerCharacter 0)))) ; if true, it means that the door needs to be open forward otherwise backward
      (Variables|DoorSetup|SetDoor%20Start "0,180.000000, 0")
      (Variables|DoorSetup|SetDoor%20Stop "0,90.000000, 0")
      (Timeline|Timeline%20-%20Door%20Driven Play)
      (else
        (Variables|DoorSetup|SetDoor%20Start "0,180.000000, 0")
        (Variables|DoorSetup|SetDoor%20Stop "0,270.000000, 0")
        (Timeline|Timeline%20-%20Door%20Driven Play)))))

(fn ConstructionScript)