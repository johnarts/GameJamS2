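; Interactable wine barrel that activates a wine component, likely a spill effect, the first time it is interacted with.
; Interact checks and sets IsDestroy on its Interactible component, so later interactions do nothing.
; It then switches on a random integer to activate one of the Wine components.
; The random range covers only Wine1 and Wine2, so the Wine3 branch never runs.
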(event EventBeginPlay)

(event Collision|EventActorBeginOverlap
  (params (OtherActor :type Actor%20Object%20Reference)))

(event EventTick
  (params (DeltaSeconds :type Float%20%28single-precision%29)))

(event EventInteract
  (bind _returnvalue (Actor|GetComponentbyClass "/Game/FirstPersonBP/Blueprints/Interactible.Interactible_C"))
  (if (not (Variables|/Game/FirstPersonBP/Blueprints/Interactible.Interactible_C|GetIsDestroy _returnvalue))
    (bind _output_get (Variables|/Game/FirstPersonBP/Blueprints/Interactible.Interactible_C|SetIsDestroy _returnvalue true))
    (switch int (Math|Random|RandomInteger 2)
      (:0
        (Components|Activation|SetActive (Variables|Default|GetWine1) _output_get false))
      (:1
        (Components|Activation|SetActive (Variables|Default|GetWine2) _output_get false))
      (:2
        (Components|Activation|SetActive (Variables|Default|GetWine3) _output_get false)))))

(fn ConstructionScript)