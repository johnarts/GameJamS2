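; Behavior Tree node for the Aubergiste AI that reacts to heard noises on each tick.
; When the AI_character controller's stimulus is tagged "Noise", it takes the last actor in the perception component's currently heard list.
; If that actor is valid, it writes the actor's location to the MoveLocation Blackboard key and switches the State key.
; Debug prints report whether the heard actor was valid.
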(event EventReceiveTickAI
  (params (OwnerController :type AI%20Controller%20Object%20Reference) (ControlledPawn :type Pawn%20Object%20Reference) (DeltaSeconds :type Float%20%28single-precision%29))
  ;[1 1 1] AI_Hear
  (bind _asai_character (Utilities|Casting|CastToAI_character OwnerController))
  (if (Utilities|Name|Equal(Name) (.tag (Variables|/Game/AI_Aubergiste/AI_character.AI_character_C|GetStimulus _asai_character)) "Noise")
    (bind _output_get (Variables|Default|SetheardObject (Class|AIPerceptionComponent|GetCurrentlyPerceivedActors (Class|AIController|GetAIPerceptionComponent OwnerController) "/Script/AIModule.AISense_Hearing")))
    (Utilities|IsValid (Utilities|Array|Get(acopy) _output_get (Utilities|Array|LastIndex _output_get))
      (:Is%20Valid
        (Development|PrintString "heard")
        (AI|BehaviorTree|SetBlackboardValueasVector (Variables|Default|GetMoveLocation) (Transformation|GetActorLocation (Utilities|Array|Get(acopy) _output_get (Utilities|Array|LastIndex _output_get))))
        (Utilities|Array|Clear _output_get)
        (Class|BTFunctionLibrary|SetBlackboardValueasEnum (Variables|Default|GetState) (Utilities|Enum|LiteralenumAI_State "NewEnumerator1")))
      (:Is%20Not%20Valid
        (Development|PrintString "not valid")))))