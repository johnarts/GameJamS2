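; Behavior tree service that drives the innkeeper AI's sight reaction to the first-person player.
; Activation resets the vision state; each tick checks whether AI perception currently sees the player.
; At full suspicion, it writes the player's location and new state to the Blackboard, copying the state to AI_character.
; Otherwise, when CanSuspicion is set, it raises suspicion inversely to player distance from LastHeardLocation, then clears the flag.
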(event EventReceiveActivationAI
  (params (OwnerController :type AI%20Controller%20Object%20Reference) (ControlledPawn :type Pawn%20Object%20Reference))
  ;[1 1 1] AI_Activation
  (Class|BTFunctionLibrary|SetBlackboardValueasEnum (Variables|Default|GetAI_StateVison) (Utilities|Enum|LiteralenumAI_State "NewEnumerator0")))

(event EventReceiveTickAI
  (params (OwnerController :type AI%20Controller%20Object%20Reference) (ControlledPawn :type Pawn%20Object%20Reference) (DeltaSeconds :type Float%20%28single-precision%29))
  (bind _returnvalue (Utilities|Enum|LiteralenumAI_State "NewEnumerator2"))
  ;[1 1 1] AI_Vision
  (Utilities|FlowControl|Sequence
    (:then_0
      (bind _outactors (Actor|GetAllActorsOfClass "/Game/Blueprint/Player/FirstPersonCharacter.FirstPersonCharacter_C"))
      (Utilities|IsValid (Utilities|Array|Get(acopy) _outactors)
        (:Is%20Valid
          (if (and true (>= (Utilities|Array|FindItem (Class|AIPerceptionComponent|GetCurrentlyPerceivedActors (Class|AIController|GetAIPerceptionComponent OwnerController) "/Script/AIModule.AISense_Sight") (Utilities|Array|Get(acopy) _outactors)) 0))
            (if (== (Variables|/Game/Blueprint/Player/FirstPersonCharacter.FirstPersonCharacter_C|Getsuspicion (Utilities|Array|Get(acopy) _outactors)) 1e+02)
              (AI|BehaviorTree|SetBlackboardValueasVector (Variables|Default|GetMoveLocation) (Transformation|GetActorLocation (Utilities|Array|Get(acopy) _outactors)))
              (Class|BTFunctionLibrary|SetBlackboardValueasEnum (Variables|Default|GetAI_StateVison) _returnvalue)
              (bind _asai_character (Utilities|Casting|CastToAI_character OwnerController))
              (Variables|/Game/Blueprint/AI_Aubergiste/AI_character.AI_character_C|SetStateCopy _asai_character _returnvalue)
              (elif (Class|BTFunctionLibrary|GetBlackboardValueasBool (Variables|Default|GetCanSuspicion))
                (Variables|/Game/Blueprint/Player/FirstPersonCharacter.FirstPersonCharacter_C|Setsuspicion (Utilities|Array|Get(acopy) _outactors) (+ (/ 5e+01 (/ (Math|Vector|VectorLength (- (Transformation|GetActorLocation (Utilities|Array|Get(acopy) _outactors)) (Class|BTFunctionLibrary|GetBlackboardValueasVector (Variables|Default|GetLastHeardLocation)))) 8e+01)) (Variables|/Game/Blueprint/Player/FirstPersonCharacter.FirstPersonCharacter_C|Getsuspicion (Utilities|Array|Get(acopy) _outactors))))
                (Class|BTFunctionLibrary|SetBlackboardValueasBool (Variables|Default|GetCanSuspicion) false)))))))))