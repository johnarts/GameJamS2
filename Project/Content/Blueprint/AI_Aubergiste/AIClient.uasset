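; AI client character that gives itself a random appearance on BeginPlay.
; It reads skin meshes, matching anim classes and a material palette from the first Global actor, drawing from that actor's shared random stream.
; One stored index pairs mesh with anim class, and a separate roll picks the slot 0 material.
; Debug prints show the names, though the palette print re-rolls and may differ from the applied material.
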(event EventBeginPlay
  (bind _mesh (Variables|Character|GetMesh))
  ;[1 1 1] SetRandomSkin
  (bind _outactors (Actor|GetAllActorsOfClass "/Game/Blueprint/Player/Global.Global_C"))
  (bind _output_get (Variables|Default|SetRandomSkinNb (Math|Integer|%(Integer) (Class|KismetMathLibrary|RandomIntegerfromStream (* (Utilities|Array|Length (Variables|/Game/Blueprint/Player/Global.Global_C|GetSkinMeshs (Utilities|Array|Get(acopy) _outactors))) 10) (Variables|/Game/Blueprint/Player/Global.Global_C|GetRandomStream (Utilities|Array|Get(acopy) _outactors))) (Utilities|Array|Length (Variables|/Game/Blueprint/Player/Global.Global_C|GetSkinMeshs (Utilities|Array|Get(acopy) _outactors))))))
  (Development|PrintString (Utilities|GetDisplayName (Utilities|Array|Get(acopy) (Variables|/Game/Blueprint/Player/Global.Global_C|GetSkinMeshs (Utilities|Array|Get(acopy) _outactors)) _output_get)))
  (Class|SkinnedMeshComponent|SetSkeletalMesh _mesh (Utilities|Array|Get(acopy) (Variables|/Game/Blueprint/Player/Global.Global_C|GetSkinMeshs (Utilities|Array|Get(acopy) _outactors)) _output_get) true)
  (Components|SkeletalMesh|SetAnimInstanceClass _mesh (Utilities|Array|Get(acopy) (Variables|/Game/Blueprint/Player/Global.Global_C|GetSkinAnims (Utilities|Array|Get(acopy) _outactors)) _output_get))
  (Rendering|Material|SetMaterial (Variables|Character|GetMesh) 0 (Utilities|Array|Get(acopy) (Variables|/Game/Blueprint/Player/Global.Global_C|GetPalette (Utilities|Array|Get(acopy) _outactors)) (Math|Integer|%(Integer) (Class|KismetMathLibrary|RandomIntegerfromStream (* (Utilities|Array|Length (Variables|/Game/Blueprint/Player/Global.Global_C|GetPalette (Utilities|Array|Get(acopy) _outactors))) 10) (Variables|/Game/Blueprint/Player/Global.Global_C|GetRandomStream (Utilities|Array|Get(acopy) _outactors))) (Utilities|Array|Length (Variables|/Game/Blueprint/Player/Global.Global_C|GetPalette (Utilities|Array|Get(acopy) _outactors))))))
  (Development|PrintString (Utilities|GetDisplayName (Utilities|Array|Get(acopy) (Variables|/Game/Blueprint/Player/Global.Global_C|GetPalette (Utilities|Array|Get(acopy) _outactors)) (Math|Integer|%(Integer) (Class|KismetMathLibrary|RandomIntegerfromStream (* (Utilities|Array|Length (Variables|/Game/Blueprint/Player/Global.Global_C|GetPalette (Utilities|Array|Get(acopy) _outactors))) 10) (Variables|/Game/Blueprint/Player/Global.Global_C|GetRandomStream (Utilities|Array|Get(acopy) _outactors))) (Utilities|Array|Length (Variables|/Game/Blueprint/Player/Global.Global_C|GetPalette (Utilities|Array|Get(acopy) _outactors))))))))

(event Collision|EventActorBeginOverlap
  (params (OtherActor :type Actor%20Object%20Reference)))

(event EventTick
  (params (DeltaSeconds :type Float%20%28single-precision%29)))

(fn ConstructionScript)