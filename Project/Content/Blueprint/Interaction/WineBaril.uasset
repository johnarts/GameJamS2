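; WineBaril is an interactable wine barrel that can be broken once, opening one of three holes at random.
; On Interact, it checks the IsDestroy flag on its Interactible, sets it, and activates a randomly chosen Hole component.
; The flag blocks any further interaction from activating another hole, and the Blueprint contains no reset logic.
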(event EventBeginPlay)

(event Collision|EventActorBeginOverlap
  (params (OtherActor :type Actor%20Object%20Reference)))

(event EventTick
  (params (DeltaSeconds :type Float%20%28single-precision%29)))

(event EventInteract
  (bind _interactible (Variables|Default|GetInteractible))
  (if (not (Variables|/Game/FirstPersonBP/Blueprints/Interactible.Interactible_C|GetIsDestroy _interactible))
    (bind _output_get (Variables|/Game/FirstPersonBP/Blueprints/Interactible.Interactible_C|SetIsDestroy _interactible true))
    (switch int (Math|Random|RandomInteger 3)
      (:0
        (Components|Activation|SetActive (Variables|Default|GetHole1) _output_get false))
      (:1
        (Components|Activation|SetActive (Variables|Default|GetHole2) _output_get false))
      (:2
        (Components|Activation|SetActive (Variables|Default|GetHole3) _output_get false)))))

(fn ConstructionScript)